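; Shotgun child of a template weapon Blueprint that overrides firing, effects and reload.
; ProcessFiring runs six debug-drawn Visibility line traces from FirePoint in random directions within a cone, ignoring the owner and applying DamagePerBullet per hit.
; PlayEffects calls a sound at the weapon's location, and Reload simply defers to the parent.
; BeginPlay calls Fire automatically once after a short delay.
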(event `self.ReceiveBeginPlay`
  (`parent.ReceiveBeginPlay`)
  (`KismetSystemLibrary.Delay` 3.0)
  (`self.Fire`))

(event `self.Reload`
  (`parent.Reload`))

(event `self.PlayEffects`
  (`GameplayStatics.PlaySoundAtLocation` null (`self.K2_GetActorLocation`) (struct) 1.0 1.0 0.0 null null null null))

(event `self.ProcessFiring`
  (bind _firepoint (`self.FirePoint`))
  (bind _returnvalue (`SceneComponent.K2_GetComponentLocation` _firepoint))
  (for _ (range 1 7)
    (bind (_outhit _returnvalue_2) (`KismetSystemLibrary.LineTraceSingle` _returnvalue (+ _returnvalue (* (`KismetMathLibrary.RandomUnitVectorInConeInDegrees` (`SceneComponent.GetForwardVector` _firepoint) 20.0) (`self.MaxDistance`))) "TraceTypeQuery1" false (`|MakeArray` (`self.GetOwner`)) "ForDuration"))
    (if _returnvalue_2
      (`GameplayStatics.ApplyDamage` (`.HitActor` (`GameplayStatics.BreakHitResult` _outhit)) (`self.DamagePerBullet`) null (`self.GetOwner`)))))

(fn `UserConstructionScript`)
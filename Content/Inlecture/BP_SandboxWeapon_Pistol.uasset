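; Sandbox pistol weapon Blueprint that fires single hitscan shots, relying on helper functions defined outside this graph.
; SandboxFire checks ammo, then either plays a sound, line traces along the fire point's forward vector and updates ammo, or reloads with a sound.
; Each shot clears CanFire and starts a HandleFireDelay timer based on rate of fire.
; BeginPlay also calls Fire after the parent's BeginPlay.
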(event `self.ReceiveBeginPlay`
  (`parent.ReceiveBeginPlay`)
  (`self.Fire`))

(event `self.SandboxFire`
  (if (`self.CanFire`)
    (`self.CheckAmmo`)
    (if true
      (`|ExecutionSequence`
        (:`then_0`
          (`self.PlaySound` null)
          (`self.LinetraceOneShot` (`SceneComponent.GetForwardVector` (`self.FirePoint`)))
          (`self.UpdateAmmo`))
        (:`then_1`
          (bind _returnvalue (`KismetSystemLibrary.K2_SetTimer` null "HandleFireDelay" (/ 1.0 (`self.RoF`))))
          (set `self.FireTimerHandle` _returnvalue)
          (set `self.CanFire` false)))
      (else
        (`self.Reload`)
        (`self.PlaySound` null)))))

(fn `UserConstructionScript`)